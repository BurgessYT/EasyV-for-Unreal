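; Serializer with ID "Focus" that turns JSON messages into camera-style focus commands for the pawn.
; Serialize parses the JSON into a string map of speed, location, rotation and target arm length.
; DataHandle converts those strings to typed values, splitting comma-separated text for vector and rotator, and passes them to the pawn's FocusMessage.
; Empty fields become -1 sentinels in every component.
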(event `self.DataHandle`
  (params (DataMap :type "Map of String to String"))
  (bind _value (`BlueprintMapLibrary.Map_Find` DataMap "speed"))
  (bind _value_2 (`BlueprintMapLibrary.Map_Find` DataMap "target_length"))
  (bind _value_3 (`BlueprintMapLibrary.Map_Find` DataMap "rotation"))
  (bind _value_4 (`BlueprintMapLibrary.Map_Find` DataMap "location"))
  (`|ExecutionSequence`
    (:`then_0`
      (if (`KismetStringLibrary.IsEmpty` _value)
        (set `self.Speed` -1.0)
        (else
          (set `self.Speed` (`KismetStringLibrary.Conv_StringToDouble` _value)))))
    (:`then_1`
      (if (`KismetStringLibrary.IsEmpty` _value_2)
        (set `self.TargetLength` -1.0)
        (else
          (set `self.TargetLength` (`KismetStringLibrary.Conv_StringToDouble` _value_2)))))
    (:`then_2`
      (if (`KismetStringLibrary.IsEmpty` _value_3)
        (set `self.Rotation` (struct :`Pitch` -1.0 :`Yaw` -1.0 :`Roll` -1.0))
        (else
          (set `self.Rotation` (`self.String To Rotation` _value_3)))))
    (:`then_3`
      (if (`KismetStringLibrary.IsEmpty` _value_4)
        (set `self.Location` (-1.0 -1.0 -1.0))
        (else
          (set `self.Location` (`self.String To Vector3D` _value_4)))))
    (:`then_4`
      (message `/BLUI/BP_Interaction_Interfaces.Focus` (`self.Pawn`) (`self.Speed`) (`self.Location`) (`self.Rotation`) (`self.TargetLength`)))))

(fn `GetSerializerID`
  (returns (Id :type Name))
  (return "Focus"))

(fn `Serialize`
  (params (Data :type String))
  (returns (DataMap :type "Map of String to String"))
  (bind _returnvalue (`BluBlueprintFunctionLibrary.ParseJSON` Data))
  (`|ExecutionSequence`
    (:`then_0`
      (bind _returnvalue_2 (`BluJsonObj.GetStringValue` _returnvalue "speed")))
    (:`then_1`
      (bind _returnvalue_3 (`BluJsonObj.GetStringValue` _returnvalue "location")))
    (:`then_2`
      (bind _returnvalue_4 (`BluJsonObj.GetStringValue` _returnvalue "rotation")))
    (:`then_3`
      (bind _returnvalue_5 (`BluJsonObj.GetStringValue` _returnvalue "target_length")))
    (:`then_4`
      (return (`|MakeMap` "speed" _returnvalue_2 "location" _returnvalue_3 "rotation" _returnvalue_4 "target_length" _returnvalue_5)))))