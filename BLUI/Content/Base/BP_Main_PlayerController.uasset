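; Main player controller driving a camera pawn while relaying mouse and key input to an embedded EasyV BluEye web widget.
; Right-drag pans along the yaw plane, left-drag rotates with clamped pitch, and MoveUp moves vertically.
; The wheel sets BP_Main_Pawn's target spring-arm length, with curves scaling zoom and vertical speed by normalized arm length.
; CallEasyV sends data to page JavaScript, while incoming EasyV custom events are only printed.
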(event `Key|AnyKey`
  (params (Key :type "Key Structure"))
  (bind _blueye (`self.GetBluEye`))
  ;[1 1 1] 任意键
  (:`Pressed`
    (`/Engine/EditorBlueprintResources/StandardMacros.IsValid` _blueye
      (:`Is Valid`
        (`BluEye.CharKeyInput` :`self` _blueye)))))

(event `Key|RightMouseButton`
  (params (Key :type "Key Structure"))
  ;[1 1 1] 鼠标右键
  (:`Pressed`
    (set `self.RightMousePress` true))
  (:`Released`
    (set `self.RightMousePress` false)))

(event `Key|LeftMouseButton`
  (params (Key :type "Key Structure"))
  (bind _blueye (`self.GetBluEye`))
  ;[1 1 1] 鼠标左键
  (:`Pressed`
    (set `self.LeftMousePress` true)
    (bind _returnvalue (`WidgetLayoutLibrary.GetMousePositionOnViewport`))
    (`/Engine/EditorBlueprintResources/StandardMacros.IsValid` _blueye
      (:`Is Valid`
        (`BluEye.TriggerLeftMouseDown` _blueye _returnvalue 1.0))))
  (:`Released`
    (set `self.LeftMousePress` false)
    (bind _returnvalue_2 (`WidgetLayoutLibrary.GetMousePositionOnViewport`))
    (`/Engine/EditorBlueprintResources/StandardMacros.IsValid` _blueye
      (:`Is Valid`
        (`BluEye.TriggerLeftMouseUp` _blueye _returnvalue_2 1.0)))))

(event `InputAxisKey|MouseWheelAxis`
  (params (AxisValue :type "Float (single-precision)"))
  (bind _blueye (`self.GetBluEye`))
  ;[1 1 1] 鼠标滚轮
  (bind _returnvalue (`WidgetLayoutLibrary.GetMousePositionOnViewport`))
  (`/Engine/EditorBlueprintResources/StandardMacros.IsValid` _blueye
    (:`Is Valid`
      (`BluEye.TriggerMouseWheel` _blueye (* (`self.MouseWheelSpeed`) AxisValue) _returnvalue 1.0))))

(event `InputAxisKey|MouseY`
  (params (AxisValue :type "Float (single-precision)"))
  ;[1 1 1] 鼠标XY
  (if (`self.RightMousePress`)
    (`Pawn.AddMovementInput` (`GameplayStatics.GetPlayerPawn` 0) (`KismetMathLibrary.GetForwardVector` (`KismetMathLibrary.MakeRotator` 0.0 0.0 (.yaw (`self.GetControlRotation`)))) (* (* AxisValue -1.0) 1.0) false)
    (`self.TriggerEasyVMouseMove` :!label _label)))

(event `InputAxis|TurnRate`
  (params (AxisValue :type "Float (single-precision)"))
  (bind _rotationspeed (`self.RotationSpeed`))
  (bind (_returnvalue_roll _returnvalue_pitch _returnvalue_yaw) (`KismetMathLibrary.BreakRotator` (`self.GetControlRotation` (`GameplayStatics.GetPlayerController` 0))))
  ;[1 1 1] 上下旋转
  (if (`self.LeftMousePress`)
    (`self.SetControlRotation` (`KismetMathLibrary.MakeRotator` 0.0 (`KismetMathLibrary.ClampAngle` (+ _returnvalue_pitch (* _rotationspeed (stale `InputAxis|LookUpRate` AxisValue))) (`self.PitchLimitMin`) (`self.PitchLimitMax`)) (+ (* AxisValue _rotationspeed) _returnvalue_yaw)) :!label _label_2)))

(event `InputAxisKey|MouseX`
  (params (AxisValue :type "Float (single-precision)"))
  ;[1 1 1] 鼠标XY
  (if (`self.RightMousePress`)
    (`Pawn.AddMovementInput` (`GameplayStatics.GetPlayerPawn` 0) (`KismetMathLibrary.GetRightVector` (`KismetMathLibrary.MakeRotator` 0.0 0.0 (.yaw (`self.GetControlRotation`)))) (* (* AxisValue -1.0) 1.0) false)
    (goto _label)))

(event `InputAxis|LookUpRate`
  (params (AxisValue :type "Float (single-precision)"))
  ;[1 1 1] 上下旋转
  (if (`self.LeftMousePress`)
    (goto _label_2)))

(event `Key|MouseScrollUp`
  (params (Key :type "Key Structure"))
  (bind _bp_main_pawn (`self.BP_Main_Pawn`))
  (bind _bp_main_pawn_2 (`self.BP_Main_Pawn`))
  ;[1 1 1] 滚轮滑动
  (:`Pressed`
    (`/Engine/EditorBlueprintResources/StandardMacros.IsValid` _bp_main_pawn_2
      (:`Is Valid`
        (set `/BLUI/Base/BP_Main_Pawn.TargetSpringArm_New` (`KismetMathLibrary.FClamp` (- (`SpringArmComponent.TargetArmLength` (`/BLUI/Base/BP_Main_Pawn.SpringArm` _bp_main_pawn_2)) (* (`CurveFloat.GetFloatValue` (`self.Zoom Intensity Curve`) (`self.Spring Arm Length Normalize`)) (`self.Zoom Speed`))) (`/BLUI/Base/BP_Main_Pawn.SpringArmLength_Min` _bp_main_pawn) (`/BLUI/Base/BP_Main_Pawn.SpringArmLength_Max` _bp_main_pawn)) (`self.BP_Main_Pawn`))))))

(event `InputAxis|MoveUp`
  (params (AxisValue :type "Float (single-precision)"))
  (bind _returnvalue (`GameplayStatics.GetPlayerPawn` 0))
  (bind (_returnvalue_x _returnvalue_y _returnvalue_z) (`KismetMathLibrary.BreakVector` (`self.GetActorUpVector` _returnvalue)))
  ;[1 1 1] 垂直移动
  (`Pawn.AddMovementInput` _returnvalue (`KismetMathLibrary.MakeVector` 0.0 0.0 _returnvalue_z) (* (* (`CurveFloat.GetFloatValue` (`self.Pan_Intensity_Curve`) (`self.Spring Arm Length Normalize`)) (`self.Pan Intensity Mouse`)) AxisValue 30.0) false))

(event `Key|MouseScrollDown`
  (params (Key :type "Key Structure"))
  (bind _bp_main_pawn (`self.BP_Main_Pawn`))
  ;[1 1 1] 滚轮滑动
  (:`Pressed`
    (`/Engine/EditorBlueprintResources/StandardMacros.IsValid` _bp_main_pawn
      (:`Is Valid`
        (set `/BLUI/Base/BP_Main_Pawn.TargetSpringArm_New` (`KismetMathLibrary.FClamp` (+ (* (`CurveFloat.GetFloatValue` (`self.Zoom Intensity Curve`) (`self.Spring Arm Length Normalize`)) (`self.Zoom Speed`)) (`SpringArmComponent.TargetArmLength` (`/BLUI/Base/BP_Main_Pawn.SpringArm` (`self.BP_Main_Pawn`)))) (`/BLUI/Base/BP_Main_Pawn.SpringArmLength_Min` _bp_main_pawn) (`/BLUI/Base/BP_Main_Pawn.SpringArmLength_Max` _bp_main_pawn)) (`self.BP_Main_Pawn`))))))

(event `self.ReceiveBeginPlay`
  ;[1 1 1] BeginPlay
  (`|ExecutionSequence`
    (:`then_0`
      (set `self.bShowMouseCursor` true)
      (`KismetSystemLibrary.ExecuteConsoleCommand` "DisableAllScreenMessages" self))
    (:`then_1`
      (bind _asbp_main_pawn (cast `/BLUI/Base/BP_Main_Pawn` (`GameplayStatics.GetPlayerPawn` 0)))
      (set `self.BP_Main_Pawn` _asbp_main_pawn))
    (:`then_2`
      (`WidgetBlueprintLibrary.SetInputMode_GameAndUIEx` self (`self.Widget_EasyV_Inside`) "DoNotLock" false))
    (:`then_3`
      ;[1 1 1] 绑定EasyV自定义消息事件
      (add `/BLUI/EasyV-Inside.EasyV_CustomEvent` (`self.Widget_EasyV_Inside`) (delegate `EasyV_CustomEvent`)))))

(event `EasyV_CustomEvent`
  (params (EventName :type String) (EventMessage :type String))
  ;[1 1 1] 绑定EasyV自定义消息事件
  (`KismetSystemLibrary.PrintString` EventName)
  (`KismetSystemLibrary.PrintString` EventMessage))

(fn `CallEasyV`
  (params (VariableName :type Name) (Data :type String))
  (`BluEye.ExecuteJSMethodWithParams` (`/BLUI/EasyV-Inside.BluEye` (`self.Widget_EasyV_Inside`)) "ue4.callback" (`|MakeArray` (`KismetStringLibrary.Concat_StrStr` "\"" (`KismetStringLibrary.Conv_NameToString` VariableName) "\"") (`KismetStringLibrary.Concat_StrStr` "\"" Data "\""))))

(fn `Spring Arm Length Normalize`
  (returns (ReturnValue :type "Float (double-precision)"))
  (bind _bp_main_pawn (`self.BP_Main_Pawn`))
  (`/Engine/EditorBlueprintResources/StandardMacros.IsValid` _bp_main_pawn
    (:`Is Valid`
      (return (`KismetMathLibrary.NormalizeToRange` (`SpringArmComponent.TargetArmLength` (`/BLUI/Base/BP_Main_Pawn.SpringArm` _bp_main_pawn)) (`/BLUI/Base/BP_Main_Pawn.SpringArmLength_Min` _bp_main_pawn) (`/BLUI/Base/BP_Main_Pawn.SpringArmLength_Max` _bp_main_pawn))))))

(fn `TriggerEasyVMouseMove`
  (bind _blueye (`self.GetBluEye`))
  (bind _returnvalue (`WidgetLayoutLibrary.GetMousePositionOnViewport`))
  (`/Engine/EditorBlueprintResources/StandardMacros.IsValid` _blueye
    (:`Is Valid`
      (`BluEye.TriggerMouseMove` _blueye _returnvalue 1.0))))

(fn `UserConstructionScript`)