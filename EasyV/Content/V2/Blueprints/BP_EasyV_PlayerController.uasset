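; Player controller that hosts the EasyV widget, creating it at 1920x1080 on BeginPlay and adding it to the viewport.
; It forwards left mouse press and release and mouse wheel axis input to the widget through its trigger functions.
; It also binds to the widget's message and log events and only prints their contents as debug strings.
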(event `self.ReceiveBeginPlay`
  (`|ExecutionSequence`
    (:`then_0`
      ;[1 1 1] 初始化
      (bind _returnvalue (`|CreateWidget` "/EasyV/V2/Blueprints/Widget/EasyV.EasyV_C" null "eyJzY3JlZW5JZCI6MjcwNTQxfQ==" (1920.0 1080.0)))
      (bind _output_get (set `self.EasyV` _returnvalue))
      (`UserWidget.AddToViewport` _output_get 0))
    (:`then_1`
      (add `/EasyV/V2/Blueprints/Widget/EasyV.EasyV Message Event` (`self.EasyV`) (delegate `EasyV Message Event_Event`))
      (add `/EasyV/V2/Blueprints/Widget/EasyV.EasyV Log Event` (`self.EasyV`) (delegate `EasyV Log Event_Event`)))))

(event `Key|LeftMouseButton`
  (params (Key :type "Key Structure"))
  (bind _easyv (`self.EasyV`))
  ;[1 1 1] 鼠标事件
  (:`Pressed`
    (`/EasyV/V2/Blueprints/Widget/EasyV.Trigger Left Mouse Down` _easyv))
  (:`Released`
    (`/EasyV/V2/Blueprints/Widget/EasyV.Trigger Left Mouse Up` _easyv)))

(event `EasyV Message Event_Event`
  (params (EventName :type String) (EventMessage :type String))
  (`KismetSystemLibrary.PrintString` (`KismetStringLibrary.Concat_StrStr` "[EasyV Cutom Event] " " Name: " EventName "   Message: " EventMessage)))

(event `EasyV Log Event_Event`
  (params (LogText :type String))
  (`KismetSystemLibrary.PrintString` (`KismetStringLibrary.Concat_StrStr` "[EasyV Cutom Event] " " Log: " LogText)))

(event `InputAxisKey|MouseWheelAxis`
  (params (AxisValue :type "Float (single-precision)"))
  ;[1 1 1] 鼠标事件
  (`/EasyV/V2/Blueprints/Widget/EasyV.Trigger Mouse Wheel` (`self.EasyV`) AxisValue))

(fn `UserConstructionScript`)