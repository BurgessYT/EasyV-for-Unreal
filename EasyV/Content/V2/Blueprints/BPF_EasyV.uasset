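; Blueprint function library with a Call EasyV helper that sends named data from Unreal to JavaScript through an EasyV widget.
; It builds a `ue4.<Name>.callback` target and calls it on the widget's EasyVCore.
; Pure strings are quoted and passed via ExecuteJSMethodWithParams, while other data is inserted raw into a script run by ExecuteJS.
; An optional debug flag prints the composed call first.
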(fn `Call EasyV`
  (params (Name :type Name) (Data :type String) (`EasyV Widget` :type "/EasyV/V2/Blueprints/Widget/EasyV Object Reference") (IsPureString :type Boolean :default true) (EnableDebugString :type Boolean))
  (bind _returnvalue (`KismetStringLibrary.Concat_StrStr` "\"" Data "\""))
  (bind _easyv_core (`/EasyV/V2/Blueprints/Widget/EasyV.EasyV_Core` `EasyV Widget`))
  (bind _returnvalue_2 (`KismetStringLibrary.Concat_StrStr` "ue4." (`KismetStringLibrary.Conv_NameToString` Name) ".callback"))
  (bind _returnvalue_3 (`KismetStringLibrary.Concat_StrStr` _returnvalue_2 "(" Data ");"))
  (if IsPureString
    (if EnableDebugString
      (`KismetSystemLibrary.PrintString` null (`KismetStringLibrary.Concat_StrStr` _returnvalue_2 "(" _returnvalue ")")))
    (`BluEye.ExecuteJSMethodWithParams` _easyv_core _returnvalue_2 (`|MakeArray` _returnvalue))
    (else
      (if EnableDebugString
        (`KismetSystemLibrary.PrintString` null _returnvalue_3))
      (`BluEye.ExecuteJS` _easyv_core _returnvalue_3))))